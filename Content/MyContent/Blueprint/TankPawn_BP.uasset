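; Player-controlled tank pawn Blueprint that handles driving, firing and camera-rig rotation.
; On BeginPlay it passes the cannon and turret references to the pawn and initializes TankMovement with both tracks.
; Move and turn axes feed intent calls on TankMovement, while the fire input calls Fire.
; Look axes rotate the azimuth gimbal in yaw and the spring arm in pitch, scaled by delta time for frame-rate independence.
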(event EventBeginPlay
  (Class|Tank|SetCanonReference (Variables|Default|GetCanon1))
  (Class|Tank|SetTurretReference (Variables|Default|GetTurret))
  (Class|TankMovementComponent|Initialize (Variables|Default|GetTankMovement) (Variables|Default|GetLeftTrack) (Variables|Default|GetRightTrack)))

(event Input|ActionEvents|InputActionFire
  (params (Key :type Key%20Structure :default "None"))
  (:Pressed
    (Class|Tank|Fire)))

(event Input|AxisEvents|InputAxisMoveForward
  (params (AxisValue :type Float%20%28single-precision%29))
  (Class|TankMovementComponent|IntendMoveForward (Variables|Default|GetTankMovement) AxisValue))

(event Input|AxisEvents|InputAxisTurnRight
  (params (AxisValue :type Float%20%28single-precision%29))
  (Class|TankMovementComponent|IntendTurnRight (Variables|Default|GetTankMovement) AxisValue))

(event Input|AxisEvents|InputAxisRotateAzimuth
  (params (AxisValue :type Float%20%28single-precision%29))
  (Transformation|AddLocalRotation (Variables|Default|GetAzimuthGimbal) (Math|Rotator|MakeRotator 0.0 0.0 (* AxisValue (Utilities|Time|GetWorldDeltaSeconds) 1e+01)) false false))

(event Input|AxisEvents|InputAxisRotateElevation
  (params (AxisValue :type Float%20%28single-precision%29))
  (Transformation|AddLocalRotation (Variables|Default|GetSpringArm) (Math|Rotator|MakeRotator 0.0 (* AxisValue (Utilities|Time|GetWorldDeltaSeconds) 1e+01) 0.0) false false))

(fn ConstructionScript)